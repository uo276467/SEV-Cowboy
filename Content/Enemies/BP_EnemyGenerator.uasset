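; BP_EnemyGenerator is a spawner actor that keeps producing actors of the configured Class inside a box area.
; On BeginPlay it starts GenerateEnemy, which spawns one actor immediately, then calls itself again after an EnemyTime delay, looping without a stop condition.
; Each spawn takes random X and Y from the Box component's scaled extent around the generator, keeping the generator's own Z.
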(event Custom|GenerateEnemy
  (bind _returnvalue (Transformation|GetActorLocation))
  (bind _box (Variables|Default|GetBox))
  (bind _returnvalue_2 (Components|Box|GetScaledBoxExtent _box))
  (bind _returnvalue_3 (Math|Random|RandomPointinBoundingBox _returnvalue _returnvalue_2))
  (Utilities|FlowControl|Sequence
    (:then_0
      (Game|SpawnActorfromClass (Variables|Default|GetClass) (Math|Transform|MakeTransform (Math|Vector|MakeVector (.x _returnvalue_3) (.y _returnvalue_3) (.Z (Math|Vector|BreakVector _returnvalue))) "0, 0, 0" "1,1,1") "Undefined" 0 0))
    (:then_1
      (Utilities|FlowControl|Delay (Variables|Default|GetEnemyTime))
      (CallFunction|GenerateEnemy))))

(event EventBeginPlay
  (bind _returnvalue (Transformation|GetActorLocation))
  (bind _box (Variables|Default|GetBox))
  (bind _returnvalue_2 (Components|Box|GetScaledBoxExtent _box))
  (bind _returnvalue_3 (Math|Random|RandomPointinBoundingBox _returnvalue _returnvalue_2))
  (CallFunction|GenerateEnemy)
  (Game|SpawnActorfromClass (Variables|Default|GetClass) (Math|Transform|MakeTransform (Math|Vector|MakeVector (.x _returnvalue_3) (.y _returnvalue_3) (.Z (Math|Vector|BreakVector _returnvalue))) "0, 0, 0" "1,1,1") "Undefined" 0 0))

(fn ConstructionScript)
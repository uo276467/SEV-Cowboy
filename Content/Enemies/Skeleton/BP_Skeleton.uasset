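; BP_Skeleton is an enemy that dies from a single projectile or explosion and drops an ammo box.
; Its overlap event runs a Sequence of casts to tell projectiles, grenades and explosions apart.
; A projectile is destroyed along with the skeleton, while a grenade only triggers its own explosion.
; Both kill paths call DropLoot after DestroyActor to spawn AmmoBoxClass at the skeleton's location.
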(event Custom|DropLoot
  (Game|SpawnActorfromClass (Variables|Default|GetAmmoBoxClass) (Math|Transform|MakeTransform (Transformation|GetActorLocation) "0, 0, 0" "1.000000,1.000000,1.000000") "Undefined" 0 0))

(event Collision|EventActorBeginOverlap
  (params (OtherActor :type Actor%20Object%20Reference))
  (Utilities|FlowControl|Sequence
    (:then_0
      (bind _asbp_projectile (Utilities|Casting|CastToBP_Projectile OtherActor))
      (Actor|DestroyActor)
      (CallFunction|DropLoot)
      (Actor|DestroyActor _asbp_projectile))
    (:then_1
      (bind _asbp_grenade (Utilities|Casting|CastToBP_Grenade OtherActor))
      (Default|CreateExplosion _asbp_grenade))
    (:then_2
      (Utilities|Casting|CastToBP_Explosion OtherActor)
      (Actor|DestroyActor)
      (CallFunction|DropLoot))))

(fn ConstructionScript)
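; AI controller for enemies that chases the player's BP_Cowboy character.
; BeginPlay caches the cowboy actor, and possession starts FollowPlayer, an AIMoveTo toward it with zero acceptance radius.
; FollowPlayer re-calls itself only when a move succeeds, with no handling for failed moves.
; Tick only checks that the cowboy is valid, and a look-at rotation node is left unused.
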(event Custom|FollowPlayer
  (AI|AIMoveTo 0 "0, 0, 0" (Variables|Default|GetCowboyPlayer) 0.0 false
    (:OnSuccess
      (CallFunction|FollowPlayer))))

(event EventBeginPlay
  (bind _returnvalue (Actor|GetActorOfClass "/Game/Cowboy/BP_Cowboy.BP_Cowboy_C"))
  (Variables|Default|SetCowboyPlayer _returnvalue))

(event EventPossess
  (params (PossessedPawn :type Pawn%20Object%20Reference))
  (CallFunction|FollowPlayer))

(event EventTick
  (params (DeltaSeconds :type Float%20%28single-precision%29))
  (bind _cowboyplayer (Variables|Default|GetCowboyPlayer)
    (:then)
    (:else)))

(fn ConstructionScript)